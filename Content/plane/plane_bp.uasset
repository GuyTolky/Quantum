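; Pilotable two-seat plane actor built on EasyFM flight model and gear components, with working ADF and VOR radio navigation.
; On authority, each tick sums all pilots' inputs (strongest throttle and brake win) into flight controls, gear and trim.
; Tick also drives flight-data-based audio, damps velocity near water level and sums NDB/VOR interface signals into needle values.
; CommandInt handles flaps, radio tuning and course selection.
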(event EventBeginPlay)

(event EventActorBeginOverlap
  (params (OtherActor :type Actor%20Object%20Reference)))

(event EventTick
  (params (DeltaSeconds :type Float%20%28single-precision%29))
  (Utilities|FlowControl|Sequence
    (:then_0
      (Networking|SwitchHasAuthority
        (:Authority
          (bind (_controls _throttle _trim _brake) (CallFunction|SumInputs))
          (CallFunction|UpdateControls _brake _throttle (.y _controls) (.z _controls) (.x _controls))
          (CallFunction|UpdateTrim DeltaSeconds DeltaSeconds _trim))))
    (:then_1
      (Networking|CanExecuteCosmeticEvents
        (:True
          (CallFunction|UpdateSound))))
    (:then_2
      (CallFunction|WaterCrash DeltaSeconds))
    (:then_3
      (CallFunction|SetFlaps))
    (:then_4
      (CallFunction|NavUpdate))))

(event EventCommandInt
  (params (Command :type multicrew_vehicle_commands%20Enum :default "NewEnumerator0") (Value :type Integer))
  (switch Utilities|FlowControl|Switch|Switchonmulticrew_vehicle_commands Command
    (:NewEnumerator0
      (Variables|Default|Setflaps_position (Math|Integer|Clamp(Integer) (+ (Variables|Default|Getflaps_position) Value) 0 3)))
    (:NewEnumerator2
      (CallFunction|TuneADF Value))
    (:NewEnumerator3
      (CallFunction|SwapFreqs))
    (:NewEnumerator4
      (CallFunction|TuneVOR Value))
    (:NewEnumerator5
      (Variables|Default|Setcourse Value))))

(fn ConstructionScript)

(fn SumInputs
  (for _array_element (Variables|Default|GetPilots)
    (Utilities|IsValid _array_element
      (:Is%20Valid
        (LocalVariables|Settotal (+ (Variables|/Game/pilot.pilot_C|GetControls_server _array_element) (LocalVariables|Gettotal)))
        (LocalVariables|Settotal_trim (+ (Variables|/Game/pilot.pilot_C|GetTrim_server _array_element) (LocalVariables|Gettotal_trim)))
        (LocalVariables|SetMaxThrottle (Math|Float|Max(Float) (LocalVariables|GetMaxThrottle) (Variables|/Game/pilot.pilot_C|GetThrottle_server _array_element)))
        (LocalVariables|SetMaxBrake (Math|Float|Max(Float) (LocalVariables|GetMaxBrake) (Variables|/Game/pilot.pilot_C|GetBrake_server _array_element))))))
  (return (LocalVariables|Gettotal) (LocalVariables|GetMaxThrottle) (LocalVariables|Gettotal_trim) (LocalVariables|GetMaxBrake)))

(fn NavUpdate
  (|updatewidgets)
  (|updatendb)
  (|updatevor
    (:Completed
      (return))))

(fn SwapFreqs
  (LocalVariables|Settemp (Variables|Default|GetVOR_frequency))
  (Variables|Default|SetVOR_frequency (Variables|Default|GetVOR_standby))
  (Variables|Default|SetVOR_standby (LocalVariables|Gettemp)))

(fn TuneVOR
  (params (B :type Integer))
  (Variables|Default|SetVOR_standby (Math|Integer|Clamp(Integer) (+ (Variables|Default|GetVOR_standby) B) 10000 13000))
  (return))

(fn TuneADF
  (params (B :type Integer))
  (Variables|Default|SetADF_frequency (Math|Integer|Clamp(Integer) (+ (Variables|Default|GetADF_frequency) B) 100 999))
  (return))

(fn SetFlaps
  (bind _easyfm_bp (Variables|Default|GetEasyFM_bp))
  (switch int (Variables|Default|Getflaps_position)
    (:Default
      _)
    (:0
      (Variables|/Script/EasyFM.easyFM|SetFlapsInput _easyfm_bp 0.0))
    (:1
      (Variables|/Script/EasyFM.easyFM|SetFlapsInput _easyfm_bp 0.3))
    (:2
      (Variables|/Script/EasyFM.easyFM|SetFlapsInput _easyfm_bp 0.6))
    (:3
      (Variables|/Script/EasyFM.easyFM|SetFlapsInput _easyfm_bp 1.0)))
  (return))

(fn WaterCrash
  (params (A :type Float%20%28double-precision%29))
  (bind _model (Variables|Default|Getmodel))
  (if (< (.z (Class|GameplayStatics|RebaseLocalOriginOntoZero (Transformation|GetWorldLocation (Variables|Default|Getmodel)))) 1e+02)
    (bind _returnvalue (Physics|GetPhysicsLinearVelocity _model "None"))
    (Class|PrimitiveComponent|SetAllPhysicsLinearVelocity _model (Math|Vector|Lerp(Vector) _returnvalue "0, 0, 0" (* A 2.0)) false))
  (return))

(fn UpdateSound
  (bind _easyfm_bp (Variables|Default|GetEasyFM_bp))
  (bind _wheel_rumble (Variables|Default|Getwheel_rumble))
  (bind _easygear (Variables|Default|GetEasyGear))
  (bind _engine_sound (Variables|Default|Getengine_sound))
  (bind _wind_sound (Variables|Default|Getwind_sound))
  (bind _easyfm_bp_2 (Variables|Default|GetEasyFM_bp))
  (bind (_velocity _truevelocity _altitude _indicatedairspeed _trueairspeed _groundspeed _mach _alpha) (Class|EasyFM|GetData _easyfm_bp_2 "GDF_Nautical" false))
  (bind _throttlepos (Variables|/Script/EasyFM.easyFM|GetThrottlePos _easyfm_bp_2))
  (bind _returnvalue (/ _groundspeed 1.5e+02))
  (bind _returnvalue_2 (/ _indicatedairspeed 2e+02))
  (bind _returnvalue_3 (Math|Float|Lerp _throttlepos _returnvalue_2 0.3))
  (bind _returnvalue_4 (Math|Float|Lerp 0.4 1.5 _returnvalue_3))
  (Audio|Components|Audio|SetPitchMultiplier _engine_sound _returnvalue_4)
  (Audio|Components|Audio|SetVolumeMultiplier _engine_sound _returnvalue_4 :!class /Script/Engine.AudioComponent)
  (Audio|Components|Audio|SetPitchMultiplier _wind_sound (Math|Float|Lerp 0.4 2.0 _returnvalue_2))
  (Audio|Components|Audio|SetVolumeMultiplier _wind_sound (Math|Float|Sqrt _returnvalue_2) :!class /Script/Engine.AudioComponent)
  (Audio|Components|Audio|SetVolumeMultiplier _wheel_rumble (* (Math|Conversions|ToFloat(Boolean) (Math|Boolean|ORBoolean (Variables|/Script/EasyFM.EasyGear|GetMainLeftOnGround _easygear) (Variables|/Script/EasyFM.EasyGear|GetMainRightOnGround _easygear) (Variables|/Script/EasyFM.EasyGear|GetNoseOnGround _easygear))) _returnvalue) :!class /Script/Engine.AudioComponent)
  (Audio|Components|Audio|SetPitchMultiplier _wheel_rumble (Math|Float|Lerp 1.0 2.0 _returnvalue))
  (Audio|Components|Audio|SetVolumeMultiplier (Variables|Default|Getflaps) (Math|Float|SelectFloat 0.0 0.5 (Math|Float|NearlyEqual(Float) (Variables|/Script/EasyFM.easyFM|GetFlapsPos _easyfm_bp) (Variables|/Script/EasyFM.easyFM|GetFlapsInput _easyfm_bp) 0.001)) :!class /Script/Engine.AudioComponent)
  (Audio|Parameter|SetFloatParameter (Variables|Default|Getalerts) "Stall" (* (/ _indicatedairspeed 2e+02) (- _alpha 12.0)) :!class /Script/Engine.AudioComponent)
  (return))

(fn UpdateTrim
  (params (B :type Float%20%28double-precision%29) (B2 :type Float%20%28double-precision%29) (InVec :type Vector))
  (bind (_x _y _z) (Math|Vector|BreakVector InVec))
  (bind _easyfm_bp (Variables|Default|GetEasyFM_bp))
  (Variables|/Script/EasyFM.easyFM|SetPitchTrimPos _easyfm_bp (Math|Float|Clamp(Float) (+ (Variables|/Script/EasyFM.easyFM|GetPitchTrimPos _easyfm_bp) (* _x B2 0.1)) -1.0))
  (Variables|/Script/EasyFM.easyFM|SetRollTrimPos _easyfm_bp (Math|Float|Clamp(Float) (+ (Variables|/Script/EasyFM.easyFM|GetRollTrimPos _easyfm_bp) (* _z B 0.1)) -1.0))
  (return))

(fn UpdateControls
  (params (brake :type Float%20%28double-precision%29) (Throttle :type Float%20%28double-precision%29) (yaw :type Float%20%28double-precision%29) (Roll :type Float%20%28double-precision%29) (Pitch :type Float%20%28double-precision%29))
  (bind _easygear (Variables|Default|GetEasyGear))
  (bind _easyfm_bp (Variables|Default|GetEasyFM_bp))
  (Class|EasyFM|SetPitchInput _easyfm_bp Pitch)
  (Class|EasyFM|SetYawInput _easyfm_bp yaw)
  (Class|EasyFM|SetRollInput _easyfm_bp Roll)
  (Class|EasyFM|SetThrottleInput _easyfm_bp Throttle)
  (Class|EasyGear|SetLeftBrakeInput _easygear brake)
  (Class|EasyGear|SetRightBrakeInput _easygear brake)
  (Class|EasyGear|SetSteeringInput _easygear yaw)
  (return))

(fn Acceleration
  (bind _easyfm_bp (Variables|Default|GetEasyFM_bp))
  (bind (_velocity _truevelocity _altitude _indicatedairspeed _trueairspeed _groundspeed _mach _alpha _slip _pitchrate _yawrate _rollrate _accelx _accely _accelz) (Class|EasyFM|GetData _easyfm_bp "GDF_UU" false))
  (return _accelx _accely _accelz _pitchrate _yawrate _rollrate))

(fn Getin
  (params (Pilot :type Pilot%20Object%20Reference))
  (bind _self self)
  (bind _seat_occupied (Variables|Default|GetSeat_occupied))
  (bind _interior (Variables|Default|Getinterior))
  (Utilities|Array|Add (Variables|Default|GetPilots) Pilot)
  (if (Utilities|Array|Get(acopy) (Variables|Default|GetSeat_occupied))
    (Utilities|Array|SetArrayElem _seat_occupied 1 true)
    (return _self _interior "crew1")
    (else
      (Utilities|Array|SetArrayElem _seat_occupied 0 true)
      (return _self _interior "crew0"))))

(fn GetOut
  (params (Pilot :type Pilot%20Object%20Reference))
  (bind _pilots (Variables|Default|GetPilots))
  (Utilities|Array|SetArrayElem (Variables|Default|GetSeat_occupied) (Utilities|Array|FindItem _pilots Pilot) false)
  (Utilities|Array|RemoveItem _pilots Pilot)
  (return true))

(fn ReadInt
  (return (Variables|Default|Getcourse)))